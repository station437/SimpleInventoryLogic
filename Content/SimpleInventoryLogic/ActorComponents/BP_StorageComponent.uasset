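; Actor component providing slot-based item storage for inventories, sized on the server at BeginPlay.
; Slot operations add with stacking, move, merge, swap, split, decrease and clear items, while take functions remove full amounts with rollback or as much as available.
; Most mutations call PostChanges to fire OnChangedStorage on non-dedicated servers; the container's OnRep fires it on clients.
; IsItemFitsToSlot gates placement in moves and splits but only checks index validity here.
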(event EventBeginPlay
  ;[1 1 1] Begin Play
  (if (Networking|IsServer)
    (Utilities|Array|Resize (Variables|Default|GetStorageContainer) (Variables|Configuration|GetStorageContainerSize))))

(fn GetStorageContainer
  (return (Variables|Default|GetStorageContainer)))

(fn GetIteminSlot
  (params (SlotIdx :type Integer))
  (Utilities|IsSlotValid SlotIdx
    (:Valid
      (return true (Utilities|Array|Get(acopy) (Variables|Default|GetStorageContainer) SlotIdx)))
    (:NotValid
      (return false ""))))

(fn AddItem
  (params (ContainerItem :type STR%20Container%20Item%20Structure))
  (if (> (Utilities|Struct|BreakSTR_ContainerItem ContainerItem) 0)
    (bind (_addedidname _addedamount _remainedamount) (Inner|AddItemtoStorage ContainerItem))
    (Inner|PostChanges)
    (return _addedidname _addedamount _remainedamount)
    (else
      (return "None" 0 0))))

(fn AddItemtoStorage
  (params (ContainerItem :type STR%20Container%20Item%20Structure))
  (bind (_idname _amount) (Utilities|Struct|BreakSTR_ContainerItem ContainerItem))
  (bind (_idname_2 _amount_2) (Utilities|Struct|BreakSTR_ContainerItem ContainerItem))
  (bind (_idname_3 _extra) (Utilities|Struct|BreakSTR_ContainerItem ContainerItem))
  (bind (_idname_4 _extra_2) (Utilities|Struct|BreakSTR_ContainerItem ContainerItem))
  (bind (_idname_5 _amount_3) (Utilities|Struct|BreakSTR_ContainerItem ContainerItem))
  (bind (_idname_6 _amount_4) (Utilities|Struct|BreakSTR_ContainerItem ContainerItem))
  (LocalVariables|SetStackSize (CallFunction|GetStackSize _idname))
  (if (and (> _amount 0) (> (Variables|Configuration|GetStorageContainerSize) 0))
    (LocalVariables|SetRemainingAmount _amount)
    (for _index (range 0 (- (Variables|Configuration|GetStorageContainerSize) 1))
      (bind _output_get (LocalVariables|SetCurrentContainerItemIdx _index))
      (bind _output_get_2 (LocalVariables|SetCurrentContainerItem (Utilities|Array|Get(acopy) (Variables|Default|GetStorageContainer) _output_get)))
      (if (Utilities|Name|NotEqual(Name) (Utilities|Struct|BreakSTR_ContainerItem _output_get_2) "None")
        (if (Inner|CheckItemIdandFreeSpace (LocalVariables|GetCurrentContainerItem) (LocalVariables|GetStackSize) (Utilities|Struct|BreakSTR_ContainerItem ContainerItem))
          (if (> (+ (Utilities|Struct|BreakSTR_ContainerItem (LocalVariables|GetCurrentContainerItem)) (LocalVariables|GetRemainingAmount)) (LocalVariables|GetStackSize))
            (LocalVariables|SetRemainingAmount (- (+ (Utilities|Struct|BreakSTR_ContainerItem (LocalVariables|GetCurrentContainerItem)) (LocalVariables|GetRemainingAmount)) (LocalVariables|GetStackSize)))
            (Utilities|Struct|SetmembersinSTR_ContainerItem (LocalVariables|GetCurrentContainerItem) (LocalVariables|GetStackSize))
            (Utilities|Array|SetArrayElem (Variables|Default|GetStorageContainer) (LocalVariables|GetCurrentContainerItemIdx) (LocalVariables|GetCurrentContainerItem))
            (else
              (Utilities|Struct|SetmembersinSTR_ContainerItem (LocalVariables|GetCurrentContainerItem) (+ (Utilities|Struct|BreakSTR_ContainerItem (LocalVariables|GetCurrentContainerItem)) (LocalVariables|GetRemainingAmount)))
              (Utilities|Array|SetArrayElem (Variables|Default|GetStorageContainer) (LocalVariables|GetCurrentContainerItemIdx) (LocalVariables|GetCurrentContainerItem))
              (return _idname_2 _amount_2 0))))
        (else
          (Utilities|Array|Add (LocalVariables|GetFreeSlotsIdx) (LocalVariables|GetCurrentContainerItemIdx)))))
    (if (> (Utilities|Array|Length (LocalVariables|GetFreeSlotsIdx)) 0)
      (for _array_element (LocalVariables|GetFreeSlotsIdx)
        (if (> (LocalVariables|GetRemainingAmount) (LocalVariables|GetStackSize))
          (LocalVariables|SetRemainingAmount (- (LocalVariables|GetRemainingAmount) (LocalVariables|GetStackSize)))
          (Utilities|Array|SetArrayElem (Variables|Default|GetStorageContainer) _array_element (Utilities|Struct|MakeSTR_ContainerItem _idname_4 (LocalVariables|GetStackSize) _extra_2))
          (else
            (Utilities|Array|SetArrayElem (Variables|Default|GetStorageContainer) _array_element (Utilities|Struct|MakeSTR_ContainerItem _idname_3 (LocalVariables|GetRemainingAmount) _extra))
            (return _idname_5 _amount_3 0)))))
    (return _idname_6 (- _amount_4 (LocalVariables|GetRemainingAmount)) (LocalVariables|GetRemainingAmount))
    (else
      (return "None" 0 0))))

(fn PostChanges
  (if (and (not (Networking|IsDedicatedServer)) (Networking|IsServer))
    (Default|CallOnChangedStorage)))

(fn CheckItemIdandFreeSpace
  (params (ContainerItem :type STR%20Container%20Item%20Structure) (StackSize :type Integer) (CheckIdName :type Name))
  (bind (_idname _amount) (Utilities|Struct|BreakSTR_ContainerItem ContainerItem))
  (return (and (Utilities|Name|Equal(Name) _idname CheckIdName) (< _amount StackSize))))

(fn MoveInsideStorage
  (params (FromSlotIdx :type Integer) (ToSlotIdx :type Integer))
  (Utilities|IsSlotValid FromSlotIdx
    (:Valid
      (Utilities|IsSlotValid ToSlotIdx
        (:Valid
          (bind _output_get (LocalVariables|SetFromContainerItem (Utilities|Array|Get(acopy) (Variables|Default|GetStorageContainer) FromSlotIdx)))
          (if (Utilities|Name|NotEqual(Name) (Utilities|Struct|BreakSTR_ContainerItem _output_get) "None")
            (bind _output_get_2 (LocalVariables|SetToContainerItem (Utilities|Array|Get(acopy) (Variables|Default|GetStorageContainer) ToSlotIdx)))
            (if (Utilities|Name|Equal(Name) (Utilities|Struct|BreakSTR_ContainerItem _output_get_2) "None")
              (if (Storage|IsItemFitstoSlot ToSlotIdx (.idname (LocalVariables|GetFromContainerItem)))
                (Utilities|Array|Swap (Variables|Default|GetStorageContainer) FromSlotIdx ToSlotIdx)
                (Inner|PostChanges))
              (elif (Utilities|Name|Equal(Name) (Utilities|Struct|BreakSTR_ContainerItem (LocalVariables|GetToContainerItem)) (Utilities|Struct|BreakSTR_ContainerItem (LocalVariables|GetFromContainerItem)))
                (bind _output_get_3 (LocalVariables|SetStackSize (CallFunction|GetStackSize (Utilities|Struct|BreakSTR_ContainerItem (LocalVariables|GetToContainerItem)))))
                (if (== _output_get_3 (Utilities|Struct|BreakSTR_ContainerItem (LocalVariables|GetToContainerItem)))
                  (Utilities|Array|Swap (Variables|Default|GetStorageContainer) FromSlotIdx ToSlotIdx)
                  (Inner|PostChanges)
                  (elif (> (+ (Utilities|Struct|BreakSTR_ContainerItem (LocalVariables|GetToContainerItem)) (Utilities|Struct|BreakSTR_ContainerItem (LocalVariables|GetFromContainerItem))) (LocalVariables|GetStackSize))
                    (Utilities|Array|SetArrayElem (Variables|Default|GetStorageContainer) ToSlotIdx (Utilities|Struct|MakeSTR_ContainerItem (.idname (LocalVariables|GetToContainerItem)) (LocalVariables|GetStackSize) (.extra (LocalVariables|GetToContainerItem))))
                    (Utilities|Array|SetArrayElem (Variables|Default|GetStorageContainer) FromSlotIdx (Utilities|Struct|MakeSTR_ContainerItem (.idname (LocalVariables|GetFromContainerItem)) (- (+ (Utilities|Struct|BreakSTR_ContainerItem (LocalVariables|GetToContainerItem)) (Utilities|Struct|BreakSTR_ContainerItem (LocalVariables|GetFromContainerItem))) (LocalVariables|GetStackSize)) (.extra (LocalVariables|GetFromContainerItem))))
                    (Inner|PostChanges)
                    (else
                      (Utilities|Array|SetArrayElem (Variables|Default|GetStorageContainer) ToSlotIdx (Utilities|Struct|MakeSTR_ContainerItem (.idname (LocalVariables|GetToContainerItem)) (+ (Utilities|Struct|BreakSTR_ContainerItem (LocalVariables|GetToContainerItem)) (Utilities|Struct|BreakSTR_ContainerItem (LocalVariables|GetFromContainerItem))) (.extra (LocalVariables|GetToContainerItem))))
                      (Utilities|Array|SetArrayElem :TargetArray (Variables|Default|GetStorageContainer) :Index FromSlotIdx)
                      (Inner|PostChanges))))
                (elif (Storage|IsItemFitstoSlot ToSlotIdx (.idname (LocalVariables|GetFromContainerItem)))
                  (if (Storage|IsItemFitstoSlot FromSlotIdx (.idname (LocalVariables|GetToContainerItem)))
                    (Utilities|Array|Swap (Variables|Default|GetStorageContainer) FromSlotIdx ToSlotIdx)
                    (Inner|PostChanges)))))))))))

(fn DivideIteminSlot
  (params (SlotIdx :type Integer) (SubtractAmount :type Integer))
  (if (> SubtractAmount 0)
    (bind _output_get (LocalVariables|SetFreeSlot (Inner|GetFreeSlot)))
    (if (>= _output_get 0)
      (bind _output_get_2 (LocalVariables|SetCurrentContainerItem (Utilities|Array|Get(acopy) (Variables|Default|GetStorageContainer) SlotIdx)))
      (if (Storage|IsItemFitstoSlot (LocalVariables|GetFreeSlot) (Utilities|Struct|BreakSTR_ContainerItem _output_get_2))
        (if (Inner|IsAmountEnough SlotIdx (+ SubtractAmount 1))
          (Utilities|Array|SetArrayElem (Variables|Default|GetStorageContainer) SlotIdx (Utilities|Struct|MakeSTR_ContainerItem (.idname (LocalVariables|GetCurrentContainerItem)) (- (.amount (LocalVariables|GetCurrentContainerItem)) SubtractAmount) (.extra (LocalVariables|GetCurrentContainerItem))))
          (Utilities|Array|SetArrayElem (Variables|Default|GetStorageContainer) (LocalVariables|GetFreeSlot) (Utilities|Struct|MakeSTR_ContainerItem (.idname (LocalVariables|GetCurrentContainerItem)) SubtractAmount (.extra (LocalVariables|GetCurrentContainerItem))))
          (Inner|PostChanges))))))

(fn GetFreeSlot
  (for _index (range 0 (- (Variables|Configuration|GetStorageContainerSize) 1))
    (if (Utilities|Name|Equal(Name) (Utilities|Struct|BreakSTR_ContainerItem (Utilities|Array|Get(acopy) (Variables|Default|GetStorageContainer) _index)) "None")
      (return _index)))
  (return -1))

(fn DecreaseAmountinSlot
  (params (SlotIdx :type Integer) (Amount :type Integer))
  (bind _storagecontainer (Variables|Default|GetStorageContainer))
  (bind _output (Utilities|Array|Get(acopy) _storagecontainer SlotIdx))
  (if (Inner|IsAmountEnough SlotIdx Amount)
    (if (== (- (.Amount (Utilities|Struct|BreakSTR_ContainerItem (Utilities|Array|Get(acopy) (Variables|Default|GetStorageContainer) SlotIdx))) Amount) 0)
      (Utilities|Array|SetArrayElem :TargetArray (Variables|Default|GetStorageContainer) :Index SlotIdx)
      (else
        (Utilities|Struct|SetmembersinSTR_ContainerItem _output (- (.Amount (Utilities|Struct|BreakSTR_ContainerItem _output)) Amount))))
    (Inner|PostChanges)
    (return true)
    (else
      (return false))))

(fn IsAmountEnough
  (params (SlotIdx :type Integer) (Amount :type Integer))
  (Utilities|IsSlotValid SlotIdx
    (:Valid
      (return (>= (Utilities|Struct|BreakSTR_ContainerItem (Utilities|Array|Get(acopy) (Variables|Default|GetStorageContainer) SlotIdx)) Amount)))
    (:NotValid
      (return false))))

(fn ClearSlot
  (params (SlotIdx :type Integer))
  (Utilities|IsSlotValid SlotIdx
    (:Valid
      (Utilities|Array|SetArrayElem :TargetArray (Variables|Default|GetStorageContainer) :Index SlotIdx)
      (Inner|PostChanges))))

(fn MoveItemtoSlot
  (params (ToSlotIdx :type Integer) (ContainerItem :type STR%20Container%20Item%20Structure))
  (bind _storagecontainer (Variables|Default|GetStorageContainer))
  (bind _output (Utilities|Array|Get(acopy) _storagecontainer ToSlotIdx))
  (Utilities|IsSlotValid ToSlotIdx
    (:Valid
      (if (Storage|IsItemFitstoSlot ToSlotIdx (.IdName (Utilities|Struct|BreakSTR_ContainerItem ContainerItem)))
        (if (Utilities|Name|Equal(Name) (.IdName (Utilities|Struct|BreakSTR_ContainerItem _output)) "None")
          (Utilities|Array|SetArrayElem (Variables|Default|GetStorageContainer) ToSlotIdx ContainerItem)
          (Inner|PostChanges)
          (return (Utilities|Struct|MakeSTR_ContainerItem (.idname ContainerItem) 0 "(bHasExtra_14_4AA2010B4BFFD576A5938B9ECAD0259F=False,Durability_5_7484D49847B030FA2DBB7C8369810CE4=0.000000,SkinId_8_DBBFE05C410E0D7E540501B7FBE82A6F=0,Submodules_12_7EA6A6E34DA8C273B1F231AD6AF80D79=)"))
          (else
            (LocalVariables|SetCurrentContainerItem _output)
            (if (Utilities|Name|Equal(Name) (.idname (LocalVariables|GetCurrentContainerItem)) (.idname ContainerItem))
              (bind _output_get (LocalVariables|SetStackSize (CallFunction|GetStackSize (.idname (LocalVariables|GetCurrentContainerItem)))))
              (if (< (.amount (LocalVariables|GetCurrentContainerItem)) _output_get)
                (if (> (+ (.amount (LocalVariables|GetCurrentContainerItem)) (.amount ContainerItem)) (LocalVariables|GetStackSize))
                  (LocalVariables|SetRemainingAmount (- (+ (.amount (LocalVariables|GetCurrentContainerItem)) (.amount ContainerItem)) (LocalVariables|GetStackSize)))
                  (Utilities|Struct|SetmembersinSTR_ContainerItem (Utilities|Array|Get(acopy) (Variables|Default|GetStorageContainer) ToSlotIdx) (LocalVariables|GetStackSize))
                  (Inner|PostChanges)
                  (return (Utilities|Struct|MakeSTR_ContainerItem (.idname ContainerItem) (LocalVariables|GetRemainingAmount) (.extra ContainerItem)))
                  (else
                    (Utilities|Struct|SetmembersinSTR_ContainerItem (Utilities|Array|Get(acopy) (Variables|Default|GetStorageContainer) ToSlotIdx) (+ (.amount (LocalVariables|GetCurrentContainerItem)) (.amount ContainerItem)))
                    (Inner|PostChanges)
                    (return (Utilities|Struct|MakeSTR_ContainerItem (.idname ContainerItem) 0 "(bHasExtra_14_4AA2010B4BFFD576A5938B9ECAD0259F=False,Durability_5_7484D49847B030FA2DBB7C8369810CE4=0.000000,SkinId_8_DBBFE05C410E0D7E540501B7FBE82A6F=0,Submodules_12_7EA6A6E34DA8C273B1F231AD6AF80D79=)"))))
                (else
                  _)))
            (Utilities|Array|SetArrayElem (Variables|Default|GetStorageContainer) ToSlotIdx ContainerItem)
            (Inner|PostChanges)
            (return (LocalVariables|GetCurrentContainerItem))))
        (else
          _)))
    (:NotValid
      _))
  (return ""))

(fn SetIteminSlot
  (params (SlotIdx :type Integer) (ContainerItem :type STR%20Container%20Item%20Structure))
  (Utilities|IsSlotValid SlotIdx
    (:Valid
      (Utilities|Array|SetArrayElem (Variables|Default|GetStorageContainer) SlotIdx ContainerItem)
      (Inner|PostChanges))))

(fn OnRepStorageContainer
  (if (not (Networking|IsServer))
    (Default|CallOnChangedStorage)))

(fn TakeFullAmount
  (params (ContainerItems :type Array%20of%20STR%20Container%20Item%20Structures))
  (for _array_element ContainerItems
    (bind (_takenidname _takenamount) (Inner|TakeFullAmountItem (.IdName (Utilities|Struct|BreakSTR_ContainerItem _array_element)) (.Amount (Utilities|Struct|BreakSTR_ContainerItem _array_element))))
    (if (> _takenamount 0)
      (Utilities|Array|Add (LocalVariables|GetTakenItems) (Utilities|Struct|MakeSTR_ContainerItem _takenidname _takenamount "(bHasExtra_14_4AA2010B4BFFD576A5938B9ECAD0259F=False,Durability_5_7484D49847B030FA2DBB7C8369810CE4=0.000000,SkinId_8_DBBFE05C410E0D7E540501B7FBE82A6F=0,Submodules_12_7EA6A6E34DA8C273B1F231AD6AF80D79=)"))
      (else
        (for _array_element_2 (LocalVariables|GetTakenItems)
          (Inner|AddItemtoStorage _array_element_2))
        (Inner|PostChanges)
        (return false))))
  (Inner|PostChanges)
  (return true))

(fn TakeFullAmountItem
  (params (IdName :type Name) (Amount :type Integer))
  (LocalVariables|SetRemainingAmount Amount)
  (for (_array_element _array_index) (Variables|Default|GetStorageContainer)
    (if (Utilities|Name|Equal(Name) (.IdName (Utilities|Struct|BreakSTR_ContainerItem _array_element)) IdName)
      (if (>= (.Amount (Utilities|Struct|BreakSTR_ContainerItem _array_element)) (LocalVariables|GetRemainingAmount))
        (if (> (- (.Amount (Utilities|Struct|BreakSTR_ContainerItem _array_element)) (LocalVariables|GetRemainingAmount)) 0)
          (Utilities|Struct|SetmembersinSTR_ContainerItem (Utilities|Array|Get(acopy) (Variables|Default|GetStorageContainer) _array_index) (- (.Amount (Utilities|Struct|BreakSTR_ContainerItem _array_element)) (LocalVariables|GetRemainingAmount)))
          (else
            (Utilities|Struct|SetmembersinSTR_ContainerItem (Utilities|Array|Get(acopy) (Variables|Default|GetStorageContainer) _array_index) "None" 0 "(bHasExtra_14_4AA2010B4BFFD576A5938B9ECAD0259F=False,Durability_5_7484D49847B030FA2DBB7C8369810CE4=0.000000,SkinId_8_DBBFE05C410E0D7E540501B7FBE82A6F=0,Submodules_12_7EA6A6E34DA8C273B1F231AD6AF80D79=)")))
        (return IdName Amount)
        (else
          (LocalVariables|SetRemainingAmount (- (LocalVariables|GetRemainingAmount) (.Amount (Utilities|Struct|BreakSTR_ContainerItem _array_element))))
          (Utilities|Struct|SetmembersinSTR_ContainerItem (Utilities|Array|Get(acopy) (Variables|Default|GetStorageContainer) _array_index) "None" 0 "(bHasExtra_14_4AA2010B4BFFD576A5938B9ECAD0259F=False,Durability_5_7484D49847B030FA2DBB7C8369810CE4=0.000000,SkinId_8_DBBFE05C410E0D7E540501B7FBE82A6F=0,Submodules_12_7EA6A6E34DA8C273B1F231AD6AF80D79=)")))))
  (if (> (- Amount (LocalVariables|GetRemainingAmount)) 0)
    (Inner|AddItemtoStorage (Utilities|Struct|MakeSTR_ContainerItem IdName (- Amount (LocalVariables|GetRemainingAmount)) "(bHasExtra_14_4AA2010B4BFFD576A5938B9ECAD0259F=False,Durability_5_7484D49847B030FA2DBB7C8369810CE4=0.000000,SkinId_8_DBBFE05C410E0D7E540501B7FBE82A6F=0,Submodules_12_7EA6A6E34DA8C273B1F231AD6AF80D79=)"))
    (return "None" 0)
    (else
      (return "None" 0))))

(fn TakeMaxAmount
  (params (ContainerItems :type Array%20of%20STR%20Container%20Item%20Structures))
  (for _array_element ContainerItems
    (bind (_takenidname _takenamount) (Inner|TakeMaxAmountItem (.IdName (Utilities|Struct|BreakSTR_ContainerItem _array_element)) (.Amount (Utilities|Struct|BreakSTR_ContainerItem _array_element))))
    (if (> _takenamount 0)
      (Utilities|Array|Add (LocalVariables|GetTakingItems) (Utilities|Struct|MakeSTR_ContainerItem _takenidname _takenamount "(bHasExtra_14_4AA2010B4BFFD576A5938B9ECAD0259F=False,Durability_5_7484D49847B030FA2DBB7C8369810CE4=0.000000,SkinId_8_DBBFE05C410E0D7E540501B7FBE82A6F=0,Submodules_12_7EA6A6E34DA8C273B1F231AD6AF80D79=)"))))
  (Inner|PostChanges)
  (return (LocalVariables|GetTakingItems)))

(fn TakeMaxAmountItem
  (params (IdName :type Name) (Amount :type Integer))
  (LocalVariables|SetRemainingAmount Amount)
  (for (_array_element _array_index) (Variables|Default|GetStorageContainer)
    (if (Utilities|Name|Equal(Name) (.IdName (Utilities|Struct|BreakSTR_ContainerItem _array_element)) IdName)
      (if (>= (.Amount (Utilities|Struct|BreakSTR_ContainerItem _array_element)) (LocalVariables|GetRemainingAmount))
        (if (> (- (.Amount (Utilities|Struct|BreakSTR_ContainerItem _array_element)) (LocalVariables|GetRemainingAmount)) 0)
          (Utilities|Struct|SetmembersinSTR_ContainerItem (Utilities|Array|Get(acopy) (Variables|Default|GetStorageContainer) _array_index) (- (.Amount (Utilities|Struct|BreakSTR_ContainerItem _array_element)) (LocalVariables|GetRemainingAmount)))
          (else
            (Utilities|Struct|SetmembersinSTR_ContainerItem (Utilities|Array|Get(acopy) (Variables|Default|GetStorageContainer) _array_index) "None" 0 "(bHasExtra_14_4AA2010B4BFFD576A5938B9ECAD0259F=False,Durability_5_7484D49847B030FA2DBB7C8369810CE4=0.000000,SkinId_8_DBBFE05C410E0D7E540501B7FBE82A6F=0,Submodules_12_7EA6A6E34DA8C273B1F231AD6AF80D79=)")))
        (return IdName Amount)
        (else
          (LocalVariables|SetRemainingAmount (- (LocalVariables|GetRemainingAmount) (.Amount (Utilities|Struct|BreakSTR_ContainerItem _array_element))))
          (LocalVariables|SetTakingAmount (+ (LocalVariables|GetTakingAmount) (.Amount (Utilities|Struct|BreakSTR_ContainerItem _array_element))))
          (Utilities|Struct|SetmembersinSTR_ContainerItem (Utilities|Array|Get(acopy) (Variables|Default|GetStorageContainer) _array_index) "None" 0 "(bHasExtra_14_4AA2010B4BFFD576A5938B9ECAD0259F=False,Durability_5_7484D49847B030FA2DBB7C8369810CE4=0.000000,SkinId_8_DBBFE05C410E0D7E540501B7FBE82A6F=0,Submodules_12_7EA6A6E34DA8C273B1F231AD6AF80D79=)")))))
  (return IdName (LocalVariables|GetTakingAmount)))

(fn ClearStorage
  (Utilities|Array|Clear (Variables|Default|GetStorageContainer))
  (Utilities|Array|Resize (Variables|Default|GetStorageContainer) (Variables|Configuration|GetStorageContainerSize)))

(fn IsItemFitstoSlot
  (params (SlotIdx :type Integer) (ItemIdName :type Name))
  (return (Utilities|Array|IsValidIndex (Variables|Default|GetStorageContainer) SlotIdx)))