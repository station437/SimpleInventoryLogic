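; BP_EquipmentComponent is an equipment storage component for the simple inventory system that restricts which items can go in which slots.
; It overrides the slot fit check so an item must pass both the parent's check and CanEquipItem for that slot.
; After the parent handles post-change processing, the server calls CallOnChangedStorageOnServer.
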(fn IsItemFitstoSlot
  (params (SlotIdx :type Integer) (ItemIdName :type Name :default "None"))
  (if (|CallParentFunction SlotIdx ItemIdName)
    (return (CallFunction|CanEquipItem ItemIdName SlotIdx))
    (else
      (return false))))

(fn PostChanges
  (|CallParentFunction)
  (if (Networking|IsServer)
    (Default|CallOnChangedStorageonServer)))